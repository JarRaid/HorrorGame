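; BP_FollowObject_01 is an actor meant to make its Cube mirror the player controller's rotation, despite the "follow" name never moving it.
; Tick's switch holds that logic in case 1: copy the rotation with a slight roll offset, flip it locally and print a debug string.
; StartFollow sets State to 1, but the switch reads a constant 0 instead of State, so that branch never runs as written.
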(event `self.ReceiveTick`
  (params (DeltaSeconds :type "Float (single-precision)"))
  (bind _returnvalue (`self.GetTransform` (`GameplayStatics.GetPlayerController` 0)))
  (switch `int` 0
    (:`1`
      (`SceneComponent.K2_SetWorldRotation` (`self.Cube`) (`KismetMathLibrary.MakeRotator` (- (.roll (.rotation _returnvalue)) 1.0) (.pitch (.rotation _returnvalue)) (.yaw (.rotation _returnvalue))) false false)
      (`SceneComponent.K2_AddLocalRotation` (`self.Cube`) (struct :`Pitch` 180.0 :`Yaw` -180.0) false false)
      (`KismetSystemLibrary.PrintString` "Hello"))))

(fn `StartFollow`
  (set `self.State` 1))

(fn `UserConstructionScript`)