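; A chasing enemy pawn that hunts the player and respawns them on contact.
; StartFollow plays a scream, then a delayed state switch lets Tick issue AI MoveTo at the player while rotating the sphere to face them.
; Reaching, hitting or overlapping the player character calls its ReSpawn and stops the chase.
; Functions change or restore movement speed, and ResetSelf returns the pawn to its starting transform and restarts the chase.
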(event `ResetSelf_Part2`
  (`GameplayStatics.PlaySoundAtLocation` "/Game/Audio/Horror_Sound_FX/Entity/SE_EntityScream.SE_EntityScream" (0.0 0.0 0.0) (struct) 1.0 1.0 0.0 null null null null)
  (`KismetSystemLibrary.Delay` 3.5)
  (set `self.State` 1))

(event `self.ReceiveBeginPlay`
  (set `self.StartSpeed` (`MovementComponent.GetMaxSpeed` (`self.FloatingPawnMovement`)))
  (set `self.StartTransform` (`KismetMathLibrary.MakeTransform` (`self.K2_GetActorLocation`) (`self.K2_GetActorRotation`))))

(event `self.ReceiveTick`
  (params (DeltaSeconds :type "Float (single-precision)"))
  (bind _returnvalue (`GameplayStatics.GetPlayerCharacter` 0))
  (bind _sphere (`self.Sphere`))
  (switch `int` (`self.State`)
    (:`1`
      (`|AIMoveTo` self (0.0 0.0 0.0) _returnvalue 0.0
        (:`then`
          (`SceneComponent.K2_SetWorldRotation` _sphere (`KismetMathLibrary.FindLookAtRotation` (`SceneComponent.K2_GetComponentLocation` _sphere) (`self.K2_GetActorLocation` _returnvalue)) false false))
        (:`OnSuccess`
          (bind _asbp_first_person_character (cast `/Game/FirstPerson/Blueprints/BP_FirstPersonCharacter` _returnvalue))
          (set `self.State` 0)
          (`/Game/FirstPerson/Blueprints/BP_FirstPersonCharacter.ReSpawn` _asbp_first_person_character))))))

(event `self.Sphere.OnComponentHit`
  (params (HitComponent :type "PrimitiveComponent Object Reference") (OtherActor :type "Actor Object Reference") (OtherComp :type "PrimitiveComponent Object Reference") (NormalImpulse :type "Vector Structure") (Hit :type "HitResult Structure (by ref)"))
  (bind _asbp_first_person_character (cast `/Game/FirstPerson/Blueprints/BP_FirstPersonCharacter` OtherActor))
  (`/Game/FirstPerson/Blueprints/BP_FirstPersonCharacter.ReSpawn` _asbp_first_person_character)
  (set `self.State` 0 :!label _label))

(event `self.Sphere.OnComponentBeginOverlap`
  (params (OverlappedComponent :type "PrimitiveComponent Object Reference") (OtherActor :type "Actor Object Reference") (OtherComp :type "PrimitiveComponent Object Reference") (OtherBodyIndex :type Integer) (bFromSweep :type Boolean) (SweepResult :type "HitResult Structure (by ref)"))
  (bind _asbp_first_person_character (cast `/Game/FirstPerson/Blueprints/BP_FirstPersonCharacter` OtherActor))
  (`/Game/FirstPerson/Blueprints/BP_FirstPersonCharacter.ReSpawn` _asbp_first_person_character)
  (goto _label))

(event `StartFollowPart02`
  (`KismetSystemLibrary.Delay` 3.5)
  (set `self.State` 1))

(fn `ChangeMaxSpeed`
  (params (Speed :type "Float (double-precision)"))
  (set `FloatingPawnMovement.MaxSpeed` Speed (`self.FloatingPawnMovement`)))

(fn `ResetMaxSpeed`
  (set `FloatingPawnMovement.MaxSpeed` (`self.StartSpeed`) (`self.FloatingPawnMovement`)))

(fn `ResetSelf`
  (bind (_starttransform_location _starttransform_rotation) (`KismetMathLibrary.BreakTransform` (`self.StartTransform`)))
  (`self.K2_SetActorLocationAndRotation` _starttransform_location _starttransform_rotation)
  (set `self.State` 0)
  (`self.StartFollow`))

(fn `StartFollow`
  (`GameplayStatics.PlaySoundAtLocation` "/Game/Audio/Horror_Sound_FX/Entity/SE_EntityScream.SE_EntityScream" (`SceneComponent.K2_GetComponentLocation` (`self.Sphere`)) (struct) 1.0 1.0 0.0 null null null null)
  (`self.StartFollowPart02`))

(fn `UserConstructionScript`)