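; BP_Curtains is a curtain that slides open when the first-person character enters its box trigger.
; The overlap sets IsOpen on itself and on a linked OtherCurtain, which points to itself when the curtain stands alone.
; Tick then shrinks the scene component's X scale over a capped timer, negated when IsFlipped mirrors the curtain, leaving it bunched open with no closing logic.
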(event `self.ReceiveTick`
  (params (DeltaSeconds :type "Float (single-precision)"))
  (bind _emptyscenecomponent (`self.emptySceneComponent`))
  (bind _returnvalue (/ (- 5.0 (`self.openTimer`)) 5.0))
  (if (`self.isOpen`)
    (bind _output_get (set `self.openTimer` (+ (`self.openTimer`) DeltaSeconds)))
    (if (> _output_get 4.0)
      (set `self.openTimer` 4.0))
    (if (`self.isFlipped`)
      (`SceneComponent.SetRelativeScale3D` _emptyscenecomponent (`KismetMathLibrary.MakeVector` (* _returnvalue -1.0) 1.0 1.0))
      (else
        (`SceneComponent.SetRelativeScale3D` _emptyscenecomponent (`KismetMathLibrary.MakeVector` _returnvalue 1.0 1.0))))))

(event `self.Box.OnComponentBeginOverlap`
  (params (OverlappedComponent :type "PrimitiveComponent Object Reference") (OtherActor :type "Actor Object Reference") (OtherComp :type "PrimitiveComponent Object Reference") (OtherBodyIndex :type Integer) (bFromSweep :type Boolean) (SweepResult :type "HitResult Structure (by ref)"))
  (cast `/Game/FirstPerson/Blueprints/BP_FirstPersonCharacter` OtherActor)
  (set `self.isOpen` true)
  (set `/Game/Blueprints_Simons/BP_Curtains.isOpen` true (`self.otherCurtain`)))

(fn `UserConstructionScript`)