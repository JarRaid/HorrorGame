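; BP_Door is an automatic single door that swings open when the first-person character enters its trigger box and closes when they leave.
; OpenDoor and CloseDoor set an IsOpen flag and switch the door mesh's collision off or back on.
; Tick counts a clamped half-second timer up or down and maps it to mesh yaw, giving a smooth reversible 90-degree swing without a Timeline.
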(event `self.ReceiveTick`
  (params (DeltaSeconds :type "Float (single-precision)"))
  (if (`self.IsOpen`)
    (bind _output_get (set `self.OpenTimer` (+ (`self.OpenTimer`) DeltaSeconds)))
    (if (> _output_get 0.5)
      (set `self.OpenTimer` 0.5))
    (else
      (bind _output_get_2 (set `self.OpenTimer` (- (`self.OpenTimer`) DeltaSeconds)))
      (if (< _output_get_2 0.0)
        (set `self.OpenTimer` 0.0))))
  (`SceneComponent.K2_SetRelativeRotation` (`self.ModularAssets_DoorSingle_231015_2024`) (`KismetMathLibrary.MakeRotator` 0.0 0.0 (* (`self.OpenTimer`) 180.0)) false false))

(event `self.Box.OnComponentBeginOverlap`
  (params (OverlappedComponent :type "PrimitiveComponent Object Reference") (OtherActor :type "Actor Object Reference") (OtherComp :type "PrimitiveComponent Object Reference") (OtherBodyIndex :type Integer) (bFromSweep :type Boolean) (SweepResult :type "HitResult Structure (by ref)"))
  (cast `/Game/FirstPerson/Blueprints/BP_FirstPersonCharacter` OtherActor)
  (`self.OpenDoor`))

(event `self.Box.OnComponentEndOverlap`
  (params (OverlappedComponent :type "PrimitiveComponent Object Reference") (OtherActor :type "Actor Object Reference") (OtherComp :type "PrimitiveComponent Object Reference") (OtherBodyIndex :type Integer))
  (cast `/Game/FirstPerson/Blueprints/BP_FirstPersonCharacter` OtherActor)
  (`self.CloseDoor`))

(fn `CloseDoor`
  (if (`self.IsOpen`)
    (set `self.IsOpen` false))
  (`PrimitiveComponent.SetCollisionEnabled` (`self.ModularAssets_DoorSingle_231015_2024`) "QueryAndPhysics"))

(fn `OpenDoor`
  (if (not (`self.IsOpen`))
    (set `self.IsOpen` true))
  (`PrimitiveComponent.SetCollisionEnabled` (`self.ModularAssets_DoorSingle_231015_2024`) "NoCollision"))

(fn `UserConstructionScript`)