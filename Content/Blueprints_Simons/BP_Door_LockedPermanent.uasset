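; BP_Door_LockedPermanent is a single door actor, named as a permanently locked variant.
; OpenDoor and CloseDoor set the IsOpen flag and switch the door mesh's collision off or back to query and physics.
; Neither function moves or animates the mesh, and the empty event graph and construction script never call them.
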(event `self.ReceiveTick`
  (params (DeltaSeconds :type "Float (single-precision)")))

(fn `CloseDoor`
  (if (`self.IsOpen`)
    (set `self.IsOpen` false))
  (`PrimitiveComponent.SetCollisionEnabled` (`self.ModularAssets_DoorSingle_231015_2024`) "QueryAndPhysics"))

(fn `OpenDoor`
  (if (not (`self.IsOpen`))
    (set `self.IsOpen` true))
  (`PrimitiveComponent.SetCollisionEnabled` (`self.ModularAssets_DoorSingle_231015_2024`) "NoCollision"))

(fn `UserConstructionScript`)