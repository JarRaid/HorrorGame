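; BP_FollowObject_02 is a pawn that follows the player character once told to start.
; StartFollow sets State to 1, and from then on Tick issues AIMoveTo toward player character 0 every frame.
; The move node's immediate output turns the Cube component to look at the player.
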(event `self.ReceiveTick`
  (params (DeltaSeconds :type "Float (single-precision)"))
  (bind _returnvalue (`GameplayStatics.GetPlayerCharacter` 0))
  (bind _cube (`self.Cube`))
  (switch `int` (`self.State`)
    (:`1`
      (`|AIMoveTo` self (0.0 0.0 0.0) _returnvalue
        (:`then`
          (`SceneComponent.K2_SetWorldRotation` _cube (`KismetMathLibrary.FindLookAtRotation` (`SceneComponent.K2_GetComponentLocation` _cube) (`self.K2_GetActorLocation` _returnvalue)) false false))))))

(fn `StartFollow`
  (set `self.State` 1))

(fn `UserConstructionScript`)