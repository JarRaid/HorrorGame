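; Physics prop actor whose FloatingObject component can be lifted into a weightless float and dropped again.
; Launch disables gravity, adds an upward velocity-change impulse and sets a slight random spin, while Land restores gravity.
; Tick caps linear speed, and the stopinair event zeroes velocities after a delay.
; Nothing in this Blueprint calls Launch, Land or stopinair, and debug prints remain.
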(event `stop in air`
  (bind _floatingobject (`self.FloatingObject`))
  ;[1 1 1] Stop function if nessesary
  (`KismetSystemLibrary.Delay` 3.0)
  (`PrimitiveComponent.SetAllPhysicsLinearVelocity` _floatingobject (0.0 0.0 0.0) false)
  (`PrimitiveComponent.SetPhysicsLinearVelocity` _floatingobject (0.0 0.0 0.0) false "None")
  (`PrimitiveComponent.SetPhysicsAngularVelocityInDegrees` _floatingobject (0.0 0.0 0.0) false "None")
  (`PrimitiveComponent.SetAllPhysicsAngularVelocityInDegrees` _floatingobject (0.0 0.0 0.0) false)
  (`KismetSystemLibrary.PrintString` "stop"))

(event `self.ReceiveTick`
  (params (DeltaSeconds :type "Float (single-precision)"))
  (bind _floatingobject (`self.FloatingObject`))
  (bind _returnvalue (`PrimitiveComponent.GetPhysicsLinearVelocity` _floatingobject "None"))
  (if (> (`KismetMathLibrary.VSize` _returnvalue) 400.0)
    (`PrimitiveComponent.SetPhysicsLinearVelocity` _floatingobject (* (`KismetMathLibrary.Normal` _returnvalue) 400.0) false "None")))

(fn `Land`
  (`PrimitiveComponent.SetEnableGravity` (`self.FloatingObject`) true))

(fn `Launch`
  (bind _floatingobject (`self.FloatingObject`))
  (`PrimitiveComponent.SetEnableGravity` _floatingobject false)
  (`PrimitiveComponent.AddVelocityChangeImpulseAtLocation` _floatingobject (0.0 0.0 60.0) (0.0 0.0 0.0) "None")
  (`PrimitiveComponent.SetPhysicsAngularVelocityInDegrees` _floatingobject (`KismetMathLibrary.MakeVector` (`KismetMathLibrary.RandomFloatInRange` -1.0 1.0) (`KismetMathLibrary.RandomFloatInRange` -1.0 1.0) (`KismetMathLibrary.RandomFloatInRange` -1.0 1.0)) false "None")
  (`KismetSystemLibrary.PrintString` (`KismetStringLibrary.Conv_VectorToString` (`PrimitiveComponent.GetPhysicsAngularVelocityInDegrees` _floatingobject "None"))))

(fn `UserConstructionScript`)