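; Lantern Blueprint with a configurable point light and optional procedural twinkle that flickers its lights and emissive material.
; Construction applies light settings and, when twinkle is enabled, creates a dynamic material on its static mesh (single mesh supported).
; A Delay on Tick periodically picks random intensity targets, clamped around the initial intensity.
; Each Tick eases lights toward the target by weighted average and writes a normalized value to the emissive parameter.
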(event `self.ReceiveBeginPlay`
  ;[1 0 0.9062] Twinkling Functions
  (if (`self.Enable Twinkling Light?`)
    (`self.TwinkleSettings`)))

(event `self.ReceiveTick`
  (params (DeltaSeconds :type "Float (single-precision)"))
  ;[1 0 0.9062] Twinkling Functions
  (if (`self.Enable Twinkling Light?`)
    (`|ExecutionSequence`
      (:`then_0`
        (`self.TwinkleUpdate`)
        (`self.DynamicMaterialUpdate`))
      (:`then_1`
        (`KismetSystemLibrary.Delay` (`self.Update Target Rate`))
        (`self.TwinkleSettings`)))))

(fn `DynamicMaterialSetup`
  ;[1 0.9862 0.4623] Automatically creates and applies the user-selected dynamic material to the mesh existing in the blueprint.This does not work if there are more than one static meshes in the blueprint.
  (if (`self.Enable Twinkling Light?`)
    (bind _returnvalue (`PrimitiveComponent.CreateDynamicMaterialInstance` (`self.GetComponentByClass` "/Script/Engine.StaticMeshComponent") (`self.Mat ID`) (`self.Mesh Material`) "None"))
    (set `self.DynamicMatLiveMaterial` _returnvalue)))

(fn `DynamicMaterialUpdate`
  (bind _intensity_dynamic_mat (`self.Intensity Dynamic Mat`))
  (if (`self.Enable Twinkling Light?`)
    (`|ExecutionSequence`
      (:`then_0`
        ;[0.2247 0.2337 1] Update Variable
        (if (not (== _intensity_dynamic_mat (`self.Intensity Dynamic Mat Last`)))
          (set `self.Intensity Dynamic Mat Last` _intensity_dynamic_mat)))
      (:`then_1`
        ;[0.2879 0.9302 1] Set [Emissive] Parameter
        (`MaterialInstanceDynamic.SetScalarParameterValue` (`self.DynamicMatLiveMaterial`) (`self.Material Instance Paramter Name`) (* (`KismetMathLibrary.WeightedMovingAverage_Float` (`self.Intensity Dynamic Mat`) (`self.Intensity Dynamic Mat Last`) (`self.Interpolation Weight (Dynamic Material)`)) (`self.Emissive Map Intensity`)))))))

(fn `LightSetup`
  (bind _pointlight (`self.PointLight`))
  (`|ExecutionSequence`
    (:`then_0`
      (`SceneComponent.SetMobility` _pointlight (`self.Mobility`)))
    (:`then_1`
      (`LightComponent.SetIntensity` _pointlight (`self.Light Initial Intensity`)))
    (:`then_2`
      (`LightComponent.SetIndirectLightingIntensity` _pointlight (`self.Light Indirect Intensity`)))
    (:`then_3`
      (`LightComponent.SetUseTemperature` _pointlight (`self.Use Temperature?`))
      (`LightComponent.SetTemperature` _pointlight (`self.Temperature`))
      (`LightComponent.SetLightColor` _pointlight (`self.Light Color`) true))
    (:`then_4`
      (`LocalLightComponent.SetAttenuationRadius` _pointlight (`self.Attenuation Radius`)))
    (:`then_5`
      (`LightComponent.SetSpecularScale` _pointlight (`self.Specular`)))))

(fn `TwinkleSettings`
  (bind _light_initial_intensity (`self.Light Initial Intensity`))
  (bind _twinkle_intensity_range (`self.Twinkle Intensity Range`))
  (bind _returnvalue (* (`self.Twinkle Clamp Min (Multiplier)`) _light_initial_intensity))
  (bind _returnvalue_2 (* (`self.Twinkle Clamp Max (Multiplier)`) _light_initial_intensity))
  (for _array_element (`self.K2_GetComponentsByClass` "/Script/Engine.LightComponent")
    (bind _intensity (`LightComponentBase.Intensity` _array_element))
    (bind _returnvalue_3 (`KismetMathLibrary.FClamp` (`KismetMathLibrary.RandomFloatInRange` (- _intensity _twinkle_intensity_range) (+ _intensity _twinkle_intensity_range)) _returnvalue _returnvalue_2))
    ;[1 1 1] Twinkling - Procedural
    ;;[0.5871 1 0.5667] Update Twinkle Intensity Target for the light components within the blueprint.
    (set `self.Intensity Light Comps` _returnvalue_3)
    ;;[1 1 1] Comment
    (set `self.Intensity Dynamic Mat` (`KismetMathLibrary.NormalizeToRange` _returnvalue_3 (* _returnvalue 0.01) _returnvalue_2))))

(fn `TwinkleUpdate`
  (if (`self.Enable Twinkling Light?`)
    ;[1 0.9365 0.2371] Sets all light components parameters to interpolate to new light intensity.
    (for _array_element (`self.K2_GetComponentsByClass` "/Script/Engine.LightComponent")
      (`LightComponent.SetIntensity` _array_element (`KismetMathLibrary.WeightedMovingAverage_Float` (`self.Intensity Light Comps`) (`LightComponentBase.Intensity` _array_element) (`self.Interpolation Weight (Lights)`))))))

(fn `UserConstructionScript`
  ;[1 1 1] Twinkle Construction Script
  (`self.LightSetup`)
  (`self.DynamicMaterialSetup`))