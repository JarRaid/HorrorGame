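; BP_Chandelier is a chandelier actor that provides a configurable point light.
; Its Construction Script copies the Blueprint's variables onto the PointLight component, setting mobility, brightness, indirect lighting, color temperature, attenuation radius and specular scale.
; The event graph holds only disabled stub events, so the Blueprint adds no runtime logic.
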(fn `UserConstructionScript`
  (bind _pointlight (`self.PointLight`))
  (`SceneComponent.SetMobility` _pointlight (`self.Mobility`))
  (`LightComponent.SetIntensity` _pointlight (`self.Light Intensity`))
  (`LightComponent.SetIndirectLightingIntensity` _pointlight (`self.Light Indirect Intensity`))
  (`LightComponent.SetTemperature` _pointlight (`self.Temperature`))
  (`LocalLightComponent.SetAttenuationRadius` _pointlight (`self.Attenuation Radius`))
  (`LightComponent.SetSpecularScale` _pointlight (`self.Specular`)))