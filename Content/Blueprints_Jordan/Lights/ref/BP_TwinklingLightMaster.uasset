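; Master Blueprint for twinkling lights that flickers a child-supplied point light and, optionally, an emissive mesh material.
; Construction configures the light, disables mesh shadows and can create a dynamic material instance.
; A delay on Tick periodically rolls clamped random intensity targets, while weighted moving averages ease the light and material parameter toward them each frame.
; Tuning comes from two phase settings structs; SetPhase2 switches to the second and hides Niagara components.
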(event `self.ReceiveBeginPlay`
  ;[1 0 0.9062] Twinkling Functions
  (if (`self.Enable Twinkling Light?`)
    (`self.TwinkleSettings`)))

(event `self.ReceiveTick`
  (params (DeltaSeconds :type "Float (single-precision)"))
  ;[1 0 0.9062] Twinkling Functions
  (if (`self.Enable Twinkling Light?`)
    (`|ExecutionSequence`
      (:`then_0`
        (`self.TwinkleUpdate`)
        (`self.DynamicMaterialUpdate`))
      (:`then_1`
        (`KismetSystemLibrary.Delay` (`self.Update Target Rate`))
        (`self.TwinkleSettings`)))))

(fn `DynamicMaterialUpdate`
  (bind _intensity_dynamic_mat (`self.Intensity Dynamic Mat`))
  (if (`self.Enable Twinkling Light?`)
    (if (`self.Apply Dynamic Material?`)
      (`|ExecutionSequence`
        (:`then_0`
          (if (not (== _intensity_dynamic_mat (`self.Intensity Dynamic Mat Last`)))
            (set `self.Intensity Dynamic Mat Last` _intensity_dynamic_mat)))
        (:`then_1`
          ;[0.2879 0.9302 1] Set [Emissive] Parameter
          (`MaterialInstanceDynamic.SetScalarParameterValue` (`self.DynamicMatLiveMaterial`) (`self.Material Instance Parameter Name`) (* (`KismetMathLibrary.WeightedMovingAverage_Float` (`self.Intensity Dynamic Mat`) (`self.Intensity Dynamic Mat Last`) (`self.Interpolation Weight (Material)`)) (`self.Emissive Map Intensity`))))))))

(fn `SetPhase2`
  (`|ExecutionSequence`
    (:`then_0`
      (set `self.Phase 2` true)
      (`self.TwinkleVariables`))
    (:`then_1`
      (for _array_element (`self.K2_GetComponentsByClass` "/Script/Niagara.NiagaraComponent")
        (`SceneComponent.SetHiddenInGame` _array_element true false)))))

(fn `Setup Dynamic Material`
  ;[1 0.9862 0.4623] Automatically creates and applies the user-selected dynamic material to the mesh existing in the blueprint.This does not work if there are more than one static meshes in the blueprint.
  (if (`self.Enable Twinkling Light?`)
    (bind _returnvalue (`PrimitiveComponent.CreateDynamicMaterialInstance` (`self.GetComponentByClass` "/Script/Engine.StaticMeshComponent") (`self.Mat ID`) (`self.Mesh Material`) "DynaMat1"))
    (set `self.DynamicMatLiveMaterial` _returnvalue)))

(fn `Setup Light`
  (bind _pointlightref (`self.PointLightRef`))
  (`|ExecutionSequence`
    (:`then_0`
      ;[1 1 1] Light Sequence
      ;;[1 1 1] Point Light
      (`LightComponent.SetUseTemperature` _pointlightref (`self.Use Temperature?`))
      (`LightComponent.SetTemperature` _pointlightref (`self.Temperature`))
      (`LightComponent.SetLightColor` _pointlightref (`self.Light Color`) true)
      (`LightComponent.SetSpecularScale` _pointlightref (`self.Specular`))
      (`LocalLightComponent.SetAttenuationRadius` _pointlightref (`self.Attenuation Radius`)))
    (:`then_1`
      (`self.TwinkleVariables`))))

(fn `Setup Mesh`
  (`PrimitiveComponent.SetCastShadow` (`self.K2_GetComponentsByClass` "/Script/Engine.StaticMeshComponent") false))

(fn `TwinkleSettings`
  (bind _twinkle_intensity_range (`self.Twinkle Intensity Range`))
  (bind _initial_intensity (`self.Initial Intensity`))
  (bind _returnvalue (* (`self.Twinkle Clamp Min (Multiplier)`) _initial_intensity))
  (bind _returnvalue_2 (* (`self.Twinkle Clamp Max (Multiplier)`) _initial_intensity))
  (bind _intensity (`LightComponentBase.Intensity` (`self.PointLightRef`)))
  (bind _returnvalue_3 (`KismetMathLibrary.FClamp` (`KismetMathLibrary.RandomFloatInRange` (- _intensity _twinkle_intensity_range) (+ _intensity _twinkle_intensity_range)) _returnvalue _returnvalue_2))
  ;[1 1 1] Twinkling - Phase 1 Settings
  ;;[0.5871 1 0.5667] Update Twinkle Intensity Target for the light components within the blueprint.
  (set `self.Intensity Light Comps` _returnvalue_3)
  ;;[1 1 1] Comment
  (set `self.Intensity Dynamic Mat` (`KismetMathLibrary.NormalizeToRange` _returnvalue_3 _returnvalue _returnvalue_2)))

(fn `TwinkleUpdate`
  (bind _pointlightref (`self.PointLightRef`))
  (if (`self.Enable Twinkling Light?`)
    ;[1 0.9365 0.2371] Sets all light components parameters to interpolate to new light intensity.
    (`LightComponent.SetIntensity` _pointlightref (`KismetMathLibrary.WeightedMovingAverage_Float` (`self.Intensity Light Comps`) (`LightComponentBase.Intensity` _pointlightref) (`self.Interpolation Weight (Lights)`)))))

(fn `TwinkleVariables`
  (if (`self.Phase 2`)
    (`self.TwinkleVariablesUpdate` (`self.Twinkle Settings (Phase 2)`))
    (else
      (`self.TwinkleVariablesUpdate` (`self.Twinkle Settings (Phase 1)`)))))

(fn `TwinkleVariablesUpdate`
  (params (`Twinkle Settings` :type "/Game/Assets/Mesh/Chandelier/TwinkleSettings Structure"))
  (bind (_initialintensity _twinkleintensityrange _emissivemapintensity _twinkleclampminmultiplier _twinkleclampmaxmultiplier _interpolationweightlights _interpolationweightmaterial _updatetargetrate _indirectlightintensity) (break `/Game/Assets/Mesh/Chandelier/TwinkleSettings` `Twinkle Settings`))
  (`|ExecutionSequence`
    (:`then_0`
      (set `self.Initial Intensity` _initialintensity))
    (:`then_1`
      (set `self.Twinkle Intensity Range` _twinkleintensityrange))
    (:`then_2`
      (set `self.Emissive Map Intensity` _emissivemapintensity))
    (:`then_3`
      (set `self.Twinkle Clamp Min (Multiplier)` _twinkleclampminmultiplier))
    (:`then_4`
      (set `self.Twinkle Clamp Max (Multiplier)` _twinkleclampmaxmultiplier))
    (:`then_5`
      (set `self.Interpolation Weight (Lights)` _interpolationweightlights))
    (:`then_6`
      (set `self.Interpolation Weight (Material)` _interpolationweightmaterial))
    (:`then_7`
      (set `self.Update Target Rate` _updatetargetrate))
    (:`then_8`
      (set `self.Indirect Intensity` _indirectlightintensity))))

(fn `TwinklingPhase2`)

(fn `UserConstructionScript`
  ;[1 1 1] Read child blueprints for light components
  (bind _output_get (set `self.PointLightRef` (`self.GetComponentByClass` "/Script/Engine.PointLightComponent")))
  ;[1 1 1] Seems redundant, but is intentional so the editor can see the initial intensity. (No need to simulate, to see the light intensity in action)
  (`LightComponent.SetIntensity` _output_get (`.InitialIntensity_32_A64370C7402EBE97CBE206A15474469F` (break `/Game/Assets/Mesh/Chandelier/TwinkleSettings` (`self.Twinkle Settings (Phase 1)`))))
  (`self.Setup Mesh`)
  (`self.Setup Light`)
  (if (`self.Apply Dynamic Material?`)
    (`self.Setup Dynamic Material`)))