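; Level actor that switches the environment to its Phase 2 state, triggered by ActivatePhase2Environment from the level Blueprint or by a debug overlap with the first-person character.
; It reveals tagged decals, swaps actors by p2show/p2hide tags and calls SetPhase2 on every twinkling light.
; Rocking horses with those tags also have their mesh collision switched between block and ignore to match visibility.
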(event `Activate Phase 2 Environment`
  ;[1 1 1] Phase 2 (Reference this in Gameplay Level Blueprint)
  (`|ExecutionSequence`
    (:`then_0`
      (`self.DecalReveal`))
    (:`then_1`
      (`self.MeshSwap`))
    (:`then_2`
      (`self.LightFlickering`))
    (:`then_3`
      (`self.RockingHorses`))))

(event `self.ReceiveActorBeginOverlap`
  (params (OtherActor :type "Actor Object Reference"))
  ;[1 1 1] Debug
  (if (`self.Trigger Box Override`)
    (cast `/Game/FirstPerson/Blueprints/BP_FirstPersonCharacter` OtherActor)
    (`self.Activate Phase 2 Environment`)))

(fn `DecalReveal`
  (bind _outactors (`GameplayStatics.GetAllActorsOfClass` "/Script/Engine.DecalActor"))
  (for _array_element _outactors
    (if (`ActorComponent.ComponentHasTag` (`DecalActor.Decal` _array_element) (`self.Phase 2 Tag`))
      (`self.SetActorHiddenInGame` _array_element false))))

(fn `LightFlickering`
  (bind _outactors (`GameplayStatics.GetAllActorsOfClass` "/Game/Blueprints_Jordan/Lights/ref/BP_TwinklingLightMaster.BP_TwinklingLightMaster_C"))
  (for _array_element _outactors
    (`/Game/Blueprints_Jordan/Lights/ref/BP_TwinklingLightMaster.SetPhase2` _array_element)))

(fn `MeshSwap`
  (`|ExecutionSequence`
    (:`then_0`
      (bind _outactors (`GameplayStatics.GetAllActorsWithTag` "p2hide"))
      (for _array_element _outactors
        (`self.SetActorHiddenInGame` _array_element true)))
    (:`then_1`
      (bind _outactors_2 (`GameplayStatics.GetAllActorsWithTag` "p2show"))
      (for _array_element_2 _outactors_2
        (`self.SetActorHiddenInGame` _array_element_2 false)))))

(fn `RockingHorses`
  (`|ExecutionSequence`
    (:`then_0`
      (bind _outactors (`GameplayStatics.GetAllActorsOfClassWithTag` "/Game/Assets/Mesh/Rocking_Horse/BP_RockingHorse.BP_RockingHorse_C" "p2show"))
      (for _array_element _outactors
        (`self.SetActorHiddenInGame` _array_element false)
        (`PrimitiveComponent.SetCollisionResponseToAllChannels` (`/Game/Assets/Mesh/Rocking_Horse/BP_RockingHorse.rockinghorse_low` _array_element) "ECR_Block")))
    (:`then_1`
      (bind _outactors_2 (`GameplayStatics.GetAllActorsOfClassWithTag` "/Game/Assets/Mesh/Rocking_Horse/BP_RockingHorse.BP_RockingHorse_C" "p2hide"))
      (for _array_element_2 _outactors_2
        (`self.SetActorHiddenInGame` _array_element_2 true)
        (`PrimitiveComponent.SetCollisionResponseToAllChannels` (`/Game/Assets/Mesh/Rocking_Horse/BP_RockingHorse.rockinghorse_low` _array_element_2) "ECR_Ignore")))))

(fn `UserConstructionScript`)